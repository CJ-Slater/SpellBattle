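; BP_HitBox is a timed spherical damage volume for spells, with radius and lifetime set from DamageInfo at construction.
; Overlapping pawns receive damage via a message, honoring owner-damage and multi-hit flags, and non-instigator kills are reported to BP_FirstPersonGameMode.
; Overlaps also call a radial impulse on the sphere component itself, a separate Hit event pushes simulating components, and sphere hits only print debug text.
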(event OnComponentBeginOverlap(Sphere)
  (params (OverlappedComponent :type Primitive%20Component%20Object%20Reference) (OtherActor :type Actor%20Object%20Reference) (OtherComp :type Primitive%20Component%20Object%20Reference) (OtherBodyIndex :type Integer) (bFromSweep :type Boolean) (SweepResult :type Hit%20Result%20Structure%20%28by%20ref%29))
  (bind _damage_info (Variables|Default|GetDamage%20Info))
  (bind _damage_info_2 (Variables|Default|GetDamage%20Info))
  (bind (_damage _damagesource) (Utilities|Struct|BreakStruct_EffectInfo _damage_info_2))
  (bind (_multihit_ _damageowner_) (Utilities|Struct|BreakStruct_EffectInfo _damage_info))
  (CallFunction|ApplyPhysics OverlappedComponent)
  (bind _aspawn (Utilities|Casting|CastToPawn OtherActor))
  (if (not (and (== _aspawn (Components|GetOwner)) (not _damageowner_)))
    (if (or _multihit_ (not (Utilities|Array|ContainsItem (Variables|Default|GetDamaged%20Character) _aspawn)))
      (bind _killed (Class|BPIHealth|ReduceHealth(Message) _aspawn (Utilities|Struct|MakeStruct_DamageSource _damage _damagesource)))
      (Utilities|Array|AddUnique (Variables|Default|GetDamaged%20Character) _aspawn)
      (if (and _killed (!= _aspawn (Game|GetInstigator)))
        (CallFunction|IncrementKilledforOwner)))))

(event OnComponentHit(Sphere)
  (params (HitComponent :type Primitive%20Component%20Object%20Reference) (OtherActor :type Actor%20Object%20Reference) (OtherComp :type Primitive%20Component%20Object%20Reference) (NormalImpulse :type Vector :default "0, 0, 0") (Hit :type Hit%20Result%20Structure%20%28by%20ref%29))
  (Development|PrintString "Hello"))

(event Custom|Increment%20Killed%20For%20Owner
  (bind _id (Class|BPIPlayerController|GetUniqueID(Message) (Pawn|GetController (Game|GetInstigator))))
  (bind _asbp_first_person_game_mode (Utilities|Casting|CastToBP_FirstPersonGameMode (Game|GetGameMode)))
  (Default|IncrementKill _asbp_first_person_game_mode _id))

(event Custom|Timeout
  (CallFunction|Destroy))

(event Custom|Destroy
  (Actor|DestroyActor))

(event EventTick
  (params (DeltaSeconds :type Float%20%28single-precision%29))
  (Utilities|FlowControl|Sequence
    (:then_0
      (bind _output_get (Variables|Default|SetDuration (- (Variables|Default|GetDuration) DeltaSeconds)))
      (if (<= _output_get 0.0)
        (CallFunction|Timeout)))))

(event Collision|EventHit
  (params (MyComp :type Primitive%20Component%20Object%20Reference) (Other :type Actor%20Object%20Reference) (OtherComp :type Primitive%20Component%20Object%20Reference) (bSelfMoved :type Boolean) (HitLocation :type Vector :default "0, 0, 0") (HitNormal :type Vector :default "0, 0, 0") (NormalImpulse :type Vector :default "0, 0, 0") (Hit :type Hit%20Result%20Structure%20%28by%20ref%29))
  (if (Physics|IsSimulatingPhysics OtherComp "None")
    (Physics|AddImpulseatLocation OtherComp (* (Transformation|GetVelocity) 1e+02) (Transformation|GetActorLocation) "None")))

(fn ConstructionScript
  (bind _damage_info (Variables|Default|GetDamage%20Info))
  (Components|Sphere|SetSphereRadius (Variables|Default|GetSphere) (.areaofeffect _damage_info) true)
  (Variables|Default|SetDuration (.duration _damage_info)))

(fn ApplyPhysics
  (params (Component :type Primitive%20Component%20Object%20Reference))
  (bind _damage_info (Variables|Default|GetDamage%20Info))
  (bind (_damage _areaofeffect) (Utilities|Struct|BreakStruct_EffectInfo _damage_info))
  (Class|PhysicsObjectBlueprintLibrary|ApplyRadialImpulse Component (Transformation|GetActorLocation) _areaofeffect (Math|Conversions|ToFloat(Integer) _damage) "RIF_Constant" false 0.0 false 0.0 1.0))