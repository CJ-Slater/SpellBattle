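; BP_PushCapsule is a short-lived spell actor that knocks overlapping physics objects and characters away from its owner, without applying damage.
; DamageInfo sets the capsule half-height and lifetime, which Tick counts down before destroying the actor.
; On overlap, simulating components get an impulse and characters are launched, skipping the owner unless DamageOwner is set.
; GetPushVelocity weakens with distance from the owner (unclamped mapping), damping vertical push and adding lift.
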(event OnComponentBeginOverlap(Collision)
  (params (OverlappedComponent :type Primitive%20Component%20Object%20Reference) (OtherActor :type Actor%20Object%20Reference) (OtherComp :type Primitive%20Component%20Object%20Reference) (OtherBodyIndex :type Integer) (bFromSweep :type Boolean) (SweepResult :type Hit%20Result%20Structure%20%28by%20ref%29))
  (Utilities|FlowControl|Sequence
    (:then_0
      (if (Physics|IsSimulatingPhysics OtherComp "None")
        (Physics|AddImpulseatLocation OtherComp (CallFunction|GetPushVelocity (Components|GetOwner OtherComp)) (Transformation|GetActorLocation) "None")))
    (:then_1
      (bind _aspawn (Utilities|Casting|CastToPawn OtherActor))
      (if (not (and (== _aspawn (Components|GetOwner)) (not (Utilities|Struct|BreakStruct_EffectInfo (Variables|Default|GetDamage%20Info)))))
        (bind _ascharacter (Utilities|Casting|CastToCharacter OtherActor))
        (Character|LaunchCharacter _ascharacter (CallFunction|GetPushVelocity _ascharacter) false false)))))

(event Custom|Timeout
  (CallFunction|Destroy))

(event Custom|Destroy
  (Actor|DestroyActor))

(event EventTick
  (params (DeltaSeconds :type Float%20%28single-precision%29))
  (Utilities|FlowControl|Sequence
    (:then_0
      (bind _output_get (Variables|Default|SetDuration (- (Variables|Default|GetDuration) DeltaSeconds)))
      (if (<= _output_get 0.0)
        (CallFunction|Timeout)))))

(fn ConstructionScript
  (bind _damage_info (Variables|Default|GetDamage%20Info))
  (Components|Capsule|SetCapsuleHalfHeight (Variables|Default|GetCollision) (.areaofeffect _damage_info) true)
  (Variables|Default|SetDuration (.duration _damage_info)))

(fn GetPushVelocity
  (params (Pushed%20Actor :type Actor%20Object%20Reference))
  (bind _returnvalue (Components|GetOwner))
  (bind _returnvalue_2 (Transformation|GetActorLocation Pushed%20Actor))
  (bind _returnvalue_3 (Transformation|GetActorLocation _returnvalue))
  (bind _returnvalue_4 (Math|Rotator|FindLookatRotation _returnvalue_3 _returnvalue_2))
  (bind _returnvalue_5 (Math|Vector|Distance(Vector) _returnvalue_2 _returnvalue_3))
  (bind _returnvalue_6 (Math|Float|MapRangeUnclamped _returnvalue_5 0.0 2.5e+03 3.2e+03 5e+02))
  (bind _returnvalue_7 (* _returnvalue_4 _returnvalue_6))
  (return (Math|Vector|MakeVector (.x _returnvalue_7) (.y _returnvalue_7) (+ (* (.z _returnvalue_7) 0.75) 2.2e+02))))