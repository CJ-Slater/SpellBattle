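; BP_PushOther is a spell that, judging by its name, pushes other characters, delegating the effect to a spawned BP_PushCapsule.
; On ServerSpellCast it gets the cast point transform from its Owner and spawns the capsule there, passing EffectInfo as damage info and the Owner as owner and instigator.
; An unconnected LaunchCharacter chain based on look direction remains in the graph and never runs.
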(event EventBeginPlay
  (|CallParentFunction) ; This node is disabled and will not be called.\nDrag off pins to build functionality.
)

(event EventTick
  (params (DeltaSeconds :type Float%20%28single-precision%29)))

(event EventServerSpellCast
  (bind _owner (Variables|Default|GetOwner))
  (bind _point (Class|BPISpellcaster|GetSpellCastPoint(Message) _owner))
  (Game|SpawnActorfromClass "/Game/Spells/Actors/BP_PushCapsule.BP_PushCapsule_C" _point "Undefined" "MultiplyWithRoot" _owner (Variables|Default|GetEffect%20Info) _owner))