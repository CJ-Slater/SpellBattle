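; BP_LightningBolt is a spell that strikes the point its owner looks at after a short charge.
; On server cast, a blocking look-at hit sets the target, and a multicast plays the charging sound there during the delay.
; A second multicast then spawns a target-point actor carrying the hit VFX and swaps charge audio for impact audio.
; The server spawns a BP_HitBox carrying the effect's damage info and finishes the cast.
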(event Custom|MC%20Charge%20FX
  (bind _returnvalue (Audio|SpawnSoundatLocation "/Game/Spells/SFX/tau_charging_Cue.tau_charging_Cue" (Variables|Default|GetTarget%20Point) "0, 0, 0" 1.0 1.0 0.9 0 0))
  (Variables|Default|SetCharge%20Sound _returnvalue))

(event Custom|MC%20Hit%20FX
  (bind _charge_sound (Variables|Default|GetCharge%20Sound))
  (bind _returnvalue (Game|SpawnActorfromClass "/Game/Spells/Actors/BP_SpellTargetPoint.BP_SpellTargetPoint_C" (Math|Conversions|ToTransform(Vector) (Variables|Default|GetTarget%20Point)) "AlwaysSpawn" "MultiplyWithRoot" 0 0))
  (Utilities|IsValid _returnvalue
    (:Is%20Valid
      (Class|NiagaraComponent|SetAsset (Variables|/Game/Spells/Actors/BP_SpellTargetPoint.BP_SpellTargetPoint_C|GetVFX _returnvalue) (Variables|Default|GetHit%20VFX) true)
      (Utilities|IsValid _charge_sound
        (:Is%20Valid
          (Audio|Components|Audio|Stop _charge_sound)
          (Components|DestroyComponent _charge_sound)
          (Audio|PlaySoundatLocation (Variables|Default|GetHit%20SFX) (Variables|Default|GetTarget%20Point) "0, 0, 0" 1.0 1.0 0.0 0 0 (Variables|Default|GetOwner) 0))))))

(event EventBeginPlay
  (|CallParentFunction) ; This node is disabled and will not be called.\nDrag off pins to build functionality.
)

(event EventTick
  (params (DeltaSeconds :type Float%20%28single-precision%29))
  (|CallParentFunction DeltaSeconds) ; This node is disabled and will not be called.\nDrag off pins to build functionality.
)

(event EventMCSpellCast)

(event EventServerSpellCast
  (bind _owner (Variables|Default|GetOwner))
  (bind (_point _hit_actor _hit_result) (Class|BPIPlayer|GetLookatPoint(Message) (Variables|Default|GetOwner)))
  (if (.bBlockingHit (Collision|BreakHitResult _hit_result))
    (Variables|Default|SetTarget%20Point _point)
    (CallFunction|MCChargeFX)
    (Utilities|FlowControl|Delay 2.0)
    (CallFunction|MCHitFX)
    (Game|SpawnActorfromClass "/Game/Spells/Actors/BP_HitBox.BP_HitBox_C" (Math|Conversions|ToTransform(Vector) (Variables|Default|GetTarget%20Point)) "AlwaysSpawn" "MultiplyWithRoot" _owner (Variables|Default|GetEffect%20Info) _owner)
    (CallFunction|FinishSpellCast)))