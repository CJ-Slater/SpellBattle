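; Base projectile spell that, on the server cast, spawns a configurable number of projectile actors from the owner's spell cast point.
; Each is rotated randomly within a spray cone around the owner's look-at direction, with a per-index offset scaled by owner forward.
; Projectiles receive owner, instigator, expiry timer and spell data; FinishSpellCast runs inside the loop, after each spawn.
; The two random spawn location/rotation helpers return zero.
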(event EventServerSpellCast
  (bind _newparam (CallFunction|GetProjectileSpawnRotation))
  (for _index (range 1 (Variables|Projectile|GetProjectile%20Count))
    (bind _point (Class|BPISpellcaster|GetSpellCastPoint(Message) (Components|GetOwner) 0.0))
    (bind _aspawn (Utilities|Casting|CastToPawn (Components|GetOwner))
      (:then
        _)
      (:CastFailed
        _))
    (bind _returnvalue (Game|SpawnActorfromClass (Variables|Default|GetProjectile%20Class) (Math|Transform|MakeTransform (+ (CallFunction|GetSpawnPointOffset _index) (+ _newparam (.Location (Math|Transform|BreakTransform _point)))) _newparam) "Undefined" "OverrideRootScale" (Components|GetOwner) (Variables|Projectile|GetProjectile%20Expiry%20Timer) _aspawn))
    (Default|PopulateDatafromCastingSpell _returnvalue self)
    (CallFunction|FinishSpellCast)))

(event EventStartSpellCast
  (params (Spell%20Cast :type Struct%20Spell%20Cast%20Structure))
  (|CallParentFunction Spell%20Cast))

(fn GetRandomProjectileSpawnLocation
  (return "0, 0, 0"))

(fn GetRandomProjectileSpawnRotation
  (return "0, 0, 0"))

(fn GetSpawnPointOffset
  (params (Projectile%20Index :type Integer))
  (return (* (Transformation|GetActorForwardVector (Components|GetOwner)) (Utilities|Array|Get(acopy) (Variables|Projectile|GetSpawn%20Point%20Offsets) Projectile%20Index))))

(fn GetProjectileSpawnRotation
  (bind _rotation (Class|BPIPlayer|GetLookatRotation(Message) (Components|GetOwner)))
  (return (Math|Rotator|MakeRotfromX (Math|Random|RandomUnitVectorinConeinDegrees (Math|Vector|GetForwardVector _rotation) (Variables|Projectile|GetMax%20Projectile%20Spray%20Angle)))))