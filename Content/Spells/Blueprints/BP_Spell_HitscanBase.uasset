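; Base Blueprint for hitscan spells, which instantly damage whatever actor the caster is looking at.
; On server cast, it gets the owner's look-at point via messages, applies damage to any hit actor and finishes the cast only when one was hit.
; Kills are credited to the owner's controller ID through the first-person game mode.
; A separate physics function applies a constant-falloff radial impulse at the target point, scaled by damage.
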(event Custom|Increment%20Killed%20For%20Owner
  (bind _id (Class|BPIPlayerController|GetUniqueID(Message) (Pawn|GetController (Variables|Default|GetOwner))))
  (bind _asbp_first_person_game_mode (Utilities|Casting|CastToBP_FirstPersonGameMode (Game|GetGameMode)))
  (Default|IncrementKill _asbp_first_person_game_mode _id))

(event EventBeginPlay
  (|CallParentFunction) ; This node is disabled and will not be called.\nDrag off pins to build functionality.
)

(event EventTick
  (params (DeltaSeconds :type Float%20%28single-precision%29)))

(event EventServerSpellCast
  (bind _effect_info (Variables|Default|GetEffect%20Info))
  (bind (_damage _damagesource) (Utilities|Struct|BreakStruct_EffectInfo _effect_info))
  (bind (_point _hit_actor) (Class|BPIPlayer|GetLookatPoint(Message) (Variables|Default|GetOwner)))
  (Variables|Default|SetTarget%20Point _point)
  (Utilities|IsValid _hit_actor
    (:Is%20Valid
      (bind _killed (Class|BPIHealth|ReduceHealth(Message) _hit_actor (Utilities|Struct|MakeStruct_DamageSource _damage _damagesource)))
      (if _killed
        (CallFunction|IncrementKilledforOwner))
      (CallFunction|FinishSpellCast))))

(fn ApplyPhysics
  (bind _effect_info (Variables|Default|GetEffect%20Info))
  (bind (_damage _areaofeffect) (Utilities|Struct|BreakStruct_EffectInfo _effect_info))
  (Class|PhysicsObjectBlueprintLibrary|ApplyRadialImpulse 0 (Variables|Default|GetTarget%20Point) _areaofeffect (Math|Conversions|ToFloat(Integer) _damage) "RIF_Constant" false 0.0 false 0.0 1.0))