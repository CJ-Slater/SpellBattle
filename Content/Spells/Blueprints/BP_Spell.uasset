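; Base spell component that performs a cast on its owning Character, destroying itself if the owner is not one.
; On BeginPlay it runs a data-update hook, then starts the cast: notify, play sound and montage, and call ServerSpellCast on authority.
; The server, multicast, held-tick and data-update hooks are empty stubs, with held effects noted as rare by design.
; FinishSpellCast schedules the component's destruction after a delay.
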(event Custom|Start%20Spell%20Cast
  (params (Spell%20Cast :type Struct%20Spell%20Cast%20Structure))
  (Default|CallOnSpellCast)
  (Audio|PlaySoundatLocation (Variables|Default|GetCast%20SFX) (Transformation|GetActorLocation (Components|GetOwner)) "0, 0, 0" 1.0 1.0 0.0 0 0 0 0)
  (bind _ascharacter (Utilities|Casting|CastToCharacter (Components|GetOwner)))
  (Animation|PlayAnimMontage _ascharacter (Variables|Default|GetCast%20Animation) 1.0 "None")
  (Networking|SwitchHasAuthority
    (:Authority
      (CallFunction|ServerSpellCast))))

(event Custom|Spell%20Cast%20Held%20Tick
  (params (Cast :type Struct%20Spell%20Cast%20Structure))
  ;[0.15 0.15 0.15 0.5] NOTE: Very few spells should actually have a held effect - I think it's funnier to have to keep shouting the spell over and over
)

(event Custom|Finish%20Spell%20Cast
  (Utilities|Time|SetTimerbyEvent (delegate Custom|End%20Spell) 1e+01))

(event Custom|Server%20Spell%20Cast)

(event Custom|MC%20Spell%20Cast)

(event Custom|End%20Spell
  (Components|DestroyComponent))

(event EventBeginPlay
  (bind _ascharacter (Utilities|Casting|CastToCharacter (Components|GetOwner))
    (:then
      (Variables|Default|SetOwner _ascharacter)
      (CallFunction|UpdateDataBasedonSpellCast)
      (CallFunction|StartSpellCast))
    (:CastFailed
      (Development|PrintString "Spell owner is not a character!")
      (Components|DestroyComponent))))

(fn UpdateDataBasedonSpellCast
  (params (Spell%20Cast :type Struct%20Spell%20Cast%20Structure)))