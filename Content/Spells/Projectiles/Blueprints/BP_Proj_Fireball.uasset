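; BP_Proj_Fireball is a fireball spell projectile that deals damage through a separately spawned hitbox when it hits another actor.
; On a hit with anything but itself, it spawns a BP_HitBox at its transform, passing the owner's damage info and instigator, then calls Timeout.
; Timeout deactivates collision, hides the mesh, swaps the Niagara emitter to the hit VFX, and destroys the actor after a short delay.
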(event OnComponentBeginOverlap(Collision)
  (params (OverlappedComponent :type Primitive%20Component%20Object%20Reference) (OtherActor :type Actor%20Object%20Reference) (OtherComp :type Primitive%20Component%20Object%20Reference) (OtherBodyIndex :type Integer) (bFromSweep :type Boolean) (SweepResult :type Hit%20Result%20Structure%20%28by%20ref%29)))

(event EventBeginPlay
  (|CallParentFunction))

(event EventTimeout
  (Components|Activation|SetActive (Variables|Default|GetCollision) false false)
  (Rendering|SetVisibility (Variables|Character|GetMesh) false false)
  (Class|NiagaraComponent|SetAsset (Variables|Default|GetNiagara%20Emitter) (Variables|Default|GetHit%20VFX) true)
  (Utilities|FlowControl|Delay 2.0)
  (Actor|DestroyActor))

(event EventTick
  (params (DeltaSeconds :type Float%20%28single-precision%29))
  (|CallParentFunction DeltaSeconds) ; This node is disabled and will not be called.\nDrag off pins to build functionality.
)

(event EventHit
  (params (MyComp :type Primitive%20Component%20Object%20Reference) (Other :type Actor%20Object%20Reference) (OtherComp :type Primitive%20Component%20Object%20Reference) (bSelfMoved :type Boolean) (HitLocation :type Vector :default "0, 0, 0") (HitNormal :type Vector :default "0, 0, 0") (NormalImpulse :type Vector :default "0, 0, 0") (Hit :type Hit%20Result%20Structure%20%28by%20ref%29))
  (if (not (== Other self))
    (Game|SpawnActorfromClass "/Game/Spells/Actors/BP_HitBox.BP_HitBox_C" (Transformation|GetActorTransform) "AlwaysSpawn" "MultiplyWithRoot" 0 (Variables|Default|GetOwner%20Damage%20Info) (Game|GetInstigator))
    (CallFunction|Timeout)))

(fn ConstructionScript
  (|CallParentFunction))