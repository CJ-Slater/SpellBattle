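; Spell projectile actor that damages pawns on hit, taking its damage, lifetime and hit sound from the casting spell.
; On spawn it registers with its instigator through interface messages, destroying itself if none exists or the projectile cap is reached.
; Hits push physics bodies and damage eligible pawns, crediting non-self kills to the game mode.
; Damaging hits and Tick-driven expiry share a Timeout that hides the mesh before delayed destruction.
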(event Custom|Timeout
  (Class|NiagaraComponent|SetAsset (Variables|Default|GetNiagara%20Emitter) (Variables|Default|GetTimeout%20VFX) true)
  (Components|Activation|SetActive (Variables|Default|GetCollision) false false)
  (Rendering|SetVisibility (Variables|Default|GetMesh) false false)
  (Utilities|FlowControl|Delay 1.0)
  (Actor|DestroyActor))

(event Custom|Populate%20Data%20From%20Casting%20Spell
  (params (Owning%20Spell :type BP%20Spell%20Projectile%20Base%20Object%20Reference))
  (Variables|Default|SetOwning%20Spell Owning%20Spell)
  (Variables|Default|SetOwner%20Damage%20Info (Variables|/Game/Spells/Blueprints/BP_Spell.BP_Spell_C|GetEffect%20Info (Variables|Default|GetOwning%20Spell)))
  (Variables|Default|SetDamage%20Type (.DamageSource (Utilities|Struct|BreakStruct_EffectInfo (Variables|/Game/Spells/Blueprints/BP_Spell.BP_Spell_C|GetEffect%20Info (Variables|Default|GetOwning%20Spell)))))
  (Variables|Default|SetExpiry%20Timer (Variables|/Game/Spells/Blueprints/BP_Spell_ProjectileBase.BP_Spell_ProjectileBase_C|GetProjectile%20Expiry%20Timer (Variables|Default|GetOwning%20Spell)))
  (Variables|Default|SetDamage (.Damage (Utilities|Struct|BreakStruct_EffectInfo (Variables|/Game/Spells/Blueprints/BP_Spell.BP_Spell_C|GetEffect%20Info (Variables|Default|GetOwning%20Spell)))))
  (Variables|Default|SetHit%20SFX (Variables|/Game/Spells/Blueprints/BP_Spell_ProjectileBase.BP_Spell_ProjectileBase_C|GetHit%20SFX (Variables|Default|GetOwning%20Spell))))

(event Custom|Increment%20Kill%20For%20Owner
  (bind _asbp_first_person_game_mode (Utilities|Casting|CastToBP_FirstPersonGameMode (Game|GetGameMode)))
  (bind _id (Class|BPIPlayerController|GetUniqueID(Message) (Pawn|GetController (Game|GetInstigator))))
  (Default|IncrementKill _asbp_first_person_game_mode _id))

(event EventBeginPlay
  (bind _returnvalue (Game|GetInstigator))
  (Utilities|IsValid _returnvalue
    (:Is%20Valid
      (bind _at_capacity (Class|BPISpellcaster|AtProjectileCapacity(Message) _returnvalue))
      (if _at_capacity
        (Actor|DestroyActor :!label _label)
        (else
          (Class|BPISpellcaster|AddActiveProjectile(Message) _returnvalue)
          (Audio|PlaySoundatLocation (Variables|Default|GetSpawn%20SFX) (Transformation|GetActorLocation) "0, 0, 0" 1.0 1.0 0.0 0 0 0 0))))
    (:Is%20Not%20Valid
      (goto _label))))

(event Collision|EventActorBeginOverlap
  (params (OtherActor :type Actor%20Object%20Reference)))

(event EventTick
  (params (DeltaSeconds :type Float%20%28single-precision%29))
  (Utilities|FlowControl|Sequence
    (:then_0
      (bind _output_get (Variables|Default|SetExpiry%20Timer (- (Variables|Default|GetExpiry%20Timer) DeltaSeconds)))
      (if (<= _output_get 0.0)
        (CallFunction|Timeout)))))

(event Collision|EventHit
  (params (MyComp :type Primitive%20Component%20Object%20Reference) (Other :type Actor%20Object%20Reference) (OtherComp :type Primitive%20Component%20Object%20Reference) (bSelfMoved :type Boolean) (HitLocation :type Vector :default "0, 0, 0") (HitNormal :type Vector :default "0, 0, 0") (NormalImpulse :type Vector :default "0, 0, 0") (Hit :type Hit%20Result%20Structure%20%28by%20ref%29))
  (Utilities|FlowControl|Sequence
    (:then_0
      (if (Physics|IsSimulatingPhysics OtherComp "None")
        (Physics|AddImpulseatLocation OtherComp (* (Transformation|GetVelocity) 1e+02) (Transformation|GetActorLocation) "None")))
    (:then_1
      (if (CallFunction|CanDamage Other)
        (CallFunction|Hit Other)
        (CallFunction|Timeout)))))

(event EventDestroyed
  (bind _returnvalue (Game|GetInstigator))
  (Utilities|IsValid _returnvalue
    (:Is%20Valid
      (Class|BPISpellcaster|RemoveActiveProjectile(Message) _returnvalue)
      (|CallParentFunction))))

(fn ConstructionScript)

(fn CanDamage
  (params (Actor :type Actor%20Object%20Reference))
  (bind _aspawn (Utilities|Casting|CastToPawn Actor)
    (:then
      (if (== _aspawn (Game|GetInstigator))
        (if (Variables|Default|GetSelf%20Damage)
          (return true))
        (else
          (return true))))
    (:CastFailed
      (return false))))

(fn Hit
  (params (Actor :type Actor%20Object%20Reference))
  (Class|NiagaraComponent|SetAsset (Variables|Default|GetNiagara%20Emitter) (Variables|Default|GetHit%20VFX) true)
  (bind _killed (Class|BPIHealth|ReduceHealth(Message) Actor (Utilities|Struct|MakeStruct_DamageSource (Variables|Default|GetDamage) (Variables|Default|GetDamage%20Type))))
  (Audio|PlaySoundatLocation (Variables|Default|GetHit%20SFX) (Transformation|GetActorLocation) "0, 0, 0" 1.0 1.0 0.0 0 0 0 0)
  (if (and _killed (!= Actor (Game|GetInstigator)))
    (CallFunction|IncrementKillforOwner)))